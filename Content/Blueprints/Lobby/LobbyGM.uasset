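; Lobby GameMode that manages players, character selection, map settings, kicks and travel to the chosen map.
; On login it registers and sets up each LobbyPC, then spawns a base character at a random PlayerStart.
; EveryoneUpdate pushes player lists and available characters to all controllers and sets start readiness from character choices.
; Map changes propagate to every controller, SwapCharacter replaces pawns, logout updates the roster, and LaunchTheGame runs servertravel by map ID.
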(event `self.K2_PostLogin`
  (params (NewPlayer :type "PlayerController Object Reference"))
  ;[1 1 1] Después de logearse, lleva la inicialización del jugador y lo spawnea
  (`/Engine/EditorBlueprintResources/ActorMacros.Switch Has Authority`
    (:`Authority`
      (`KismetArrayLibrary.Array_Add` (`self.AllPlayerControllers`) NewPlayer)
      (bind _outactors (`GameplayStatics.GetAllActorsOfClass` "/Script/Engine.PlayerStart"))
      (set `self.SpawnPoints` _outactors)
      (bind _asgame_info_instance (cast `/Game/Blueprints/AllLevels/GameInfoInstance` (`GameplayStatics.GetGameInstance`)))
      (set `self.ServerName` (`/Game/Blueprints/AllLevels/GameInfoInstance.ServerName` _asgame_info_instance))
      (set `self.MaxPlayers` (`/Game/Blueprints/AllLevels/GameInfoInstance.MaxPlayers` _asgame_info_instance))
      (bind _aslobby_pc (cast `/Game/Blueprints/Lobby/LobbyPC` NewPlayer))
      (`/Game/Blueprints/Lobby/LobbyPC.InitialSetup` _aslobby_pc)
      (`/Game/Blueprints/Lobby/LobbyPC.SetUpLobbyMenu` _aslobby_pc (`KismetTextLibrary.Conv_StringToText` (`self.ServerName`)))
      (`/Game/Blueprints/Lobby/LobbyPC.UpdateLobbySettings` _aslobby_pc (`self.GM_MapImage`) (`self.GM_MapName`) (`self.GM_MapTime`))
      (`self.RespawnPlayer` NewPlayer))))

(event `RespawnPlayer`
  (params (PlayerControllerRef :type "PlayerController Object Reference"))
  (bind _returnvalue (`Controller.K2_GetPawn` PlayerControllerRef))
  (bind _spawnpoints (`self.SpawnPoints`))
  ;[1 1 1] Spawnea al jugador como personaje base al llegar al Lobby / Ordena a todos a actualizar sus lobbys
  (`/Engine/EditorBlueprintResources/StandardMacros.IsValid` _returnvalue
    (:`Is Valid`
      (`self.K2_DestroyActor` _returnvalue))
    (:`Is Not Valid`
      _))
  (bind _returnvalue_2 (`|SpawnActorFromClass` "/Game/Blueprints/Characters/0_Base.0_Base_C" (`self.GetTransform` (`|GetArrayItem` _spawnpoints (`KismetMathLibrary.RandomIntegerInRange` 0 (- (`KismetArrayLibrary.Array_Length` _spawnpoints) 1)))) "Undefined" "OverrideRootScale" null null))
  (`Controller.Possess` PlayerControllerRef _returnvalue_2)
  (`self.EveryoneUpdate`))

(event `EveryoneUpdate`
  (bind _allplayercontrollers (`self.AllPlayerControllers`))
  ;[1 1 1] Actualiza la información de todos los lobbys de los jugadores
  (bind _output_get (set `self.CurrentPlayers` (`KismetArrayLibrary.Array_Length` (`self.AllPlayerControllers`))))
  (if (> _output_get 0)
    (`KismetArrayLibrary.Array_Clear` (`self.ConnectedPlayers`))
    (for _array_element _allplayercontrollers
      (bind _aslobby_pc (cast `/Game/Blueprints/Lobby/LobbyPC` _array_element))
      (`KismetArrayLibrary.Array_Add` (`self.ConnectedPlayers`) (`/Game/Blueprints/Lobby/LobbyPC.PlayerSettings` _aslobby_pc))
      (`/Game/Blueprints/Lobby/LobbyPC.UpdateNumberOfPlayers` _aslobby_pc (`self.CurrentPlayers`) (`self.MaxPlayers`)))
    (for _array_element_2 _allplayercontrollers
      (bind _aslobby_pc_2 (cast `/Game/Blueprints/Lobby/LobbyPC` _array_element_2))
      (`/Game/Blueprints/Lobby/LobbyPC.AddPlayerInfo` _aslobby_pc_2 (`self.ConnectedPlayers`))
      (`/Game/Blueprints/Lobby/LobbyPC.UpdateAvailableCharacters` _aslobby_pc_2 (`self.AvailableCharacters`))
      (`self.AddToKickList`))
    (for _array_element_3 (`self.ConnectedPlayers`)
      (if (== (`.MyPlayerCharacter_12_A4AD884A48E170611FD99CA877FF6A69` (break `/Game/Blueprints/AllLevels/PlayerInfo` _array_element_3)) "/Game/Blueprints/Characters/0_Base.0_Base_C")
        (set `self.CanWeStart?` false)
        (`self.CannotStartGame`)
        (else
          (set `self.CanWeStart?` true))))))

(event `ServerUpdateGameSettings`
  (params (MapImage :type "Texture2D Object Reference") (MapName :type Text) (MapTime :type Text) (MapId :type Integer))
  ;[1 1 1] Servidor ha hecho cambios, decir a cada cliente que actualice la información del lobby
  (set `self.GM_MapImage` MapImage)
  (set `self.GM_MapName` MapName)
  (set `self.GM_MapTime` MapTime)
  (set `self.GM_MapId` MapId)
  (for _array_element (`self.AllPlayerControllers`)
    (bind _aslobby_pc (cast `/Game/Blueprints/Lobby/LobbyPC` _array_element))
    (`/Game/Blueprints/Lobby/LobbyPC.UpdateLobbySettings` _aslobby_pc (`self.GM_MapImage`) (`self.GM_MapName`) (`self.GM_MapTime`))))

(event `LaunchTheGame`
  (bind _returnvalue (`GameplayStatics.GetPlayerController` 0))
  ;[1 1 1] Lanza el juego en base a la selección del mapa
  (switch `int` (`self.GM_MapId`)
    (:`0`
      (`KismetSystemLibrary.ExecuteConsoleCommand` "servertravel /Game/Maps/Map01" _returnvalue))
    (:`1`
      (`KismetSystemLibrary.ExecuteConsoleCommand` "servertravel /Game/Maps/Map02" _returnvalue))))

(event `AddToKickList`
  ;[1 1 1] Añae jugador a lista de kickeo en el caso excepcional que la ventana de kickeo estuviera abierta
  (bind _aslobby_pc (cast `/Game/Blueprints/Lobby/LobbyPC` (`GameplayStatics.GetPlayerController` 0)))
  (bind _lobbymenuwb (`/Game/Blueprints/Lobby/LobbyPC.LobbyMenuWB` _aslobby_pc))
  (`/Engine/EditorBlueprintResources/StandardMacros.IsValid` _lobbymenuwb
    (:`Is Valid`
      (bind _gamesettings (`/Game/UI/Lobby/LobbyMenu.GameSettings` _lobbymenuwb))
      (if (`Widget.IsVisible` _gamesettings)
        (`/Game/UI/Lobby/GameSettings.FillPlayersWindow` _gamesettings)))))

(event `YouHaveBeenKicked`
  (params (PlayerId :type Integer))
  ;[1 1 1] Kickea el jugador seleccionado
  (`/Game/Blueprints/Lobby/LobbyPC.Kicked` (cast `/Game/Blueprints/Lobby/LobbyPC` (`|GetArrayItem` (`self.AllPlayerControllers`) PlayerId) :!pure true)))

(event `self.K2_OnLogout`
  (params (ExitingController :type "Controller Object Reference"))
  (bind _allplayercontrollers (`self.AllPlayerControllers`))
  ;[1 1 1] Cuando un jugador sale de la partida, el mismo o por kickeo...
  (for (_array_element _array_index) _allplayercontrollers
    (if (== _array_element ExitingController)
      (break)))
  (bind _aslobby_pc (cast `/Game/Blueprints/Lobby/LobbyPC` (`|GetArrayItem` _allplayercontrollers _array_index)))
  (`KismetArrayLibrary.Array_Set` (`self.AvailableCharacters`) (`/Game/Blueprints/Lobby/LobbyPC.SelectedCharacter` _aslobby_pc))
  (`KismetArrayLibrary.Array_Remove` (`self.AllPlayerControllers`) _array_index)
  (`KismetArrayLibrary.Array_Remove` (`self.ConnectedPlayers`) _array_index)
  (`self.EveryoneUpdate`))

(event `CannotStartGame`)

(event `SwapCharacter`
  (params (PlayerController :type "PlayerController Object Reference") (CharacterClass :type "Character Class Reference") (ChangedStatus :type Boolean))
  (bind _returnvalue (`Controller.K2_GetPawn` PlayerController))
  (bind _spawnpoints (`self.SpawnPoints`))
  ;[1 1 1] Cambia el personaje actual con el seleccionado en la pantalla de seleccion de personaje
  (if (not ChangedStatus)
    (`/Engine/EditorBlueprintResources/StandardMacros.IsValid` _returnvalue
      (:`Is Valid`
        (`self.K2_DestroyActor` _returnvalue))
      (:`Is Not Valid`
        _))
    (bind _returnvalue_2 (`|SpawnActorFromClass` CharacterClass (`self.GetTransform` (`|GetArrayItem` _spawnpoints (`KismetMathLibrary.RandomIntegerInRange` 0 (- (`KismetArrayLibrary.Array_Length` _spawnpoints) 1)))) "Undefined" "OverrideRootScale" null null))
    (`Controller.Possess` PlayerController _returnvalue_2)))

(fn `UserConstructionScript`)