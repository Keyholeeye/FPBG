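; Gameplay GameMode for a turn-based multiplayer session that spawns players and manages whose turn it is.
; RespawnPlayer spawns and possesses each chosen character at a random PlayerStart; once all session players are in, the server shuffles the turn order.
; GiveTurn sets each controller's waiting flag, updates its turn list and starts a looping one-second countdown, which passes the turn at zero.
; Logout triggers session teardown through the GameInstance.
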(event `StartTurnCountdown`
  ;[1 1 1] Inicia la cuenta atrás según empieza el nuevo turno
  (set `self.RemainingTurnTime` (`/Game/Blueprints/AllLevels/GameInfoInstance.CurrSessionTurnTime` (`self.GameInstanceRef`)))
  (`KismetSystemLibrary.K2_SetTimer` null "TurnTimerDecrement" 1.0 true))

(event `PassTurn`
  (params (FromPlayer :type "PlayerController Object Reference"))
  ;[1 1 1] Pasa turno cuando jugador que ya lo tenía lo indica. Comprueba que quien solicita el cambio de turno sea el jugador que tenía el turno y no otro...
  (if (`KismetSystemLibrary.IsServer`)
    (`/Engine/EditorBlueprintResources/StandardMacros.IsValid` FromPlayer
      (:`Is Valid`
        (if (== (`|GetArrayItem` (`self.TurnOrder`) (`self.CurrTurnIndex`)) (`KismetArrayLibrary.Array_Find` (`self.AllPlayerControllers`) FromPlayer))
          (bind _result (`/Engine/EditorBlueprintResources/StandardMacros.IncrementInt` (`self.CurrTurnIndex`) :!label _label)
            (:`  `
              (if (> _result (- (`KismetArrayLibrary.Array_Length` (`self.AllPlayerControllers`)) 1))
                (set `self.CurrTurnIndex` 0)
                (else
                  (set `self.CurrTurnIndex` _result)))
              (`self.GiveTurn` (`self.CurrTurnIndex`))))))
      (:`Is Not Valid`
        (goto _label)))))

(event `GiveTurn`
  (params (Index :type Integer))
  (bind _turnorder (`self.TurnOrder`))
  ;[1 1 1] El host asigna turno a jugador, al resto los pone en espera
  (`|ExecutionSequence`
    (:`then_0`
      (for (_ _array_index) _turnorder
        (if (== Index _array_index)
          (bind _asgameplay_pc (cast `/Game/Blueprints/Gameplay/GameplayPC` (`|GetArrayItem` (`self.AllPlayerControllers`) (`|GetArrayItem` _turnorder _array_index)) :!pure true))
          (set `/Game/Blueprints/Gameplay/GameplayPC.IsWaitingTurn?` false _asgameplay_pc)
          (else
            (set `/Game/Blueprints/Gameplay/GameplayPC.IsWaitingTurn?` true _asgameplay_pc)))
        (`/Game/Blueprints/Gameplay/GameplayPC.UpdateTurnPlayerList` _asgameplay_pc 1 Index)))
    (:`then_1`
      (`self.StartTurnCountdown`))))

(event `self.ReceiveBeginPlay`
  ;[1 1 1] Al generarse este GameMode, obtiene referencia a la Instancia de Juego primero...
  (bind _asgame_info_instance (cast `/Game/Blueprints/AllLevels/GameInfoInstance` (`GameplayStatics.GetGameInstance`)))
  (set `self.GameInstanceRef` _asgame_info_instance))

(event `SetPlayersTurnOrder`
  (bind _turnorder (`self.TurnOrder`))
  (bind _allplayercontrollers (`self.AllPlayerControllers`))
  ;[1 1 1] Establece orden de turnos de los jugadores, simplemente mezcla el orden de los PC que ya existen en la partida
  (`|ExecutionSequence`
    (:`then_0`
      (for (_ _array_index) _allplayercontrollers
        (`KismetArrayLibrary.Array_Add` _turnorder _array_index)
        (`KismetArrayLibrary.Array_Shuffle` _turnorder)))
    (:`then_1`
      (for _array_element _allplayercontrollers
        (bind _asgameplay_pc (cast `/Game/Blueprints/Gameplay/GameplayPC` _array_element))
        (`/Game/Blueprints/Gameplay/GameplayPC.FillTurnSwitcher` _asgameplay_pc (`/Game/Blueprints/AllLevels/GameInfoInstance.CurrSessionPlayerInfos` (`self.GameInstanceRef`)) (`self.TurnOrder`))
        (`/Game/Blueprints/Gameplay/GameplayPC.UpdateTurnPlayerList` _asgameplay_pc 1 0))
      (bind _output_get (set `self.CurrTurnIndex` 0))
      (`self.GiveTurn` _output_get))))

(event `RespawnPlayer`
  (params (PlayerController :type "PlayerController Object Reference") (PlayerCharacter :type "Character Class Reference"))
  (bind _returnvalue (`Controller.K2_GetPawn` PlayerController))
  (bind _spawnpoints (`self.SpawnPoints`))
  ;[1 1 1] Spawnea el jugador con su personaje seleccionado, lo añade a la lista de PlayerControllers
  (`|ExecutionSequence`
    (:`then_0`
      (`KismetArrayLibrary.Array_Add` (`self.AllPlayerControllers`) PlayerController))
    (:`then_1`
      (bind _outactors (`GameplayStatics.GetAllActorsOfClass` "/Script/Engine.PlayerStart"))
      (set `self.SpawnPoints` _outactors)
      (`/Engine/EditorBlueprintResources/StandardMacros.IsValid` _returnvalue
        (:`Is Valid`
          (`self.K2_DestroyActor` _returnvalue))
        (:`Is Not Valid`
          _))
      (bind _returnvalue_2 (`|SpawnActorFromClass` PlayerCharacter (`self.GetTransform` (`|GetArrayItem` _spawnpoints (`KismetMathLibrary.RandomIntegerInRange` 0 (- (`KismetArrayLibrary.Array_Length` _spawnpoints) 1)))) "Undefined" "OverrideRootScale" null null))
      (`Controller.Possess` PlayerController _returnvalue_2)
      ;;[1 1 1] Esto quiero que se ejecute solo en el host
      (if (`KismetSystemLibrary.IsServer`)
        (bind _allplayersin_ (`self.CheckIfAllPlayersIn`))
        (if _allplayersin_
          (`self.SetPlayersTurnOrder`))))))

(event `self.K2_OnLogout`
  (params (ExitingController :type "Controller Object Reference"))
  ;[1 1 1] Evento cuando el jugador sale de partida, destruye sesión
  (bind _asgameplay_pc (cast `/Game/Blueprints/Gameplay/GameplayPC` ExitingController))
  (`/Game/Blueprints/AllLevels/GameInfoInstance.DestroySessionCaller` (cast `/Game/Blueprints/AllLevels/GameInfoInstance` (`GameplayStatics.GetGameInstance`) :!pure true) _asgameplay_pc))

(fn `CheckIfAllPlayersIn`
  (returns (`AllPlayersIn?` :type Boolean))
  (if (== (`KismetArrayLibrary.Array_Length` (`self.AllPlayerControllers`)) (`/Game/Blueprints/AllLevels/GameInfoInstance.CurrSessionNumOfPlayers` (`self.GameInstanceRef`)))
    (return true)
    (else
      (return false))))

(fn `TurnTimerDecrement`
  (bind _output_get (set `self.RemainingTurnTime` (- (`self.RemainingTurnTime`) 1)))
  (`|ExecutionSequence`
    (:`then_0`
      (`KismetSystemLibrary.PrintString` (`KismetStringLibrary.Conv_IntToString` _output_get)))
    (:`then_1`
      (if (== _output_get 0)
        (`self.PassTurn` null)))))

(fn `UserConstructionScript`)