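; Game instance that drives the front-end menus, online session flow, error reporting and player settings save.
; Menu and loading widgets are mostly created once and cached, while the server menu is rebuilt each time; a missing save opens Options with a welcome message.
; Hosting creates a session and opens the Lobby as a listen server; joining uses the selected search result.
; Session, network and travel failures appear in an error dialog.
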(event `SetCurrSessionTurnTime`
  (params (TurnTime :type Integer))
  (set `self.CurrSessionTurnTime` TurnTime))

(event `SaveGameCheck`
  ;[1 1 1] Comprueba si hay un archivo de guardado previo
  (bind _returnvalue (`GameplayStatics.DoesSaveGameExist` (`self.PlayerSettingsSave`)))
  (if _returnvalue
    (`self.ShowMainMenu`)
    (set `self.CreatedSaveFile?` true)
    (else
      (`self.ShowOptionsMenu`)
      (set `PlayerController.bShowMouseCursor` true (`GameplayStatics.GetPlayerController` 0)))))

(event `SetCurrPlayerInfos`
  (params (PInfos :type "Array of /Game/Blueprints/AllLevels/PlayerInfo Structure"))
  (set `self.CurrSessionPlayerInfos` PInfos))

(event `SetCurrSessionNumOfPlayers`
  (params (NumOfPlayers :type Integer))
  (set `self.CurrSessionNumOfPlayers` NumOfPlayers))

(event `ShowMainMenu`
  (bind _returnvalue (`GameplayStatics.GetPlayerController` 0))
  ;[1 1 1] Muestra el menú principal y el cursor del ratón
  (`/Engine/EditorBlueprintResources/StandardMacros.IsValid` (`self.MainMenuWB`) ; El widget se ha creado? Si es así, lo muestra, sino, lo crea
    (:`Is Valid`
      _)
    (:`Is Not Valid`
      (bind _returnvalue_2 (`|CreateWidget` "/Game/UI/MainMenu/MainMenu.MainMenu_C" _returnvalue))
      (set `self.MainMenuWB` _returnvalue_2)))
  (`UserWidget.AddToViewport` (`self.MainMenuWB`) 0)
  (set `PlayerController.bShowMouseCursor` true _returnvalue))

(event `ShowLoadingScreen`
  ;[1 1 1] Pantalla de carga
  (`/Engine/EditorBlueprintResources/StandardMacros.IsValid` (`self.LoadingScreenWB`)
    (:`Is Valid`
      _)
    (:`Is Not Valid`
      (bind _returnvalue (`|CreateWidget` "/Game/UI/AllLevels/LoadingScreen.LoadingScreen_C" (`GameplayStatics.GetPlayerController` 0)))
      (set `self.LoadingScreenWB` _returnvalue)))
  (`UserWidget.AddToViewport` (`self.LoadingScreenWB`) 0))

(event `self.HandleNetworkError`
  (params (FailureType :type "ENetworkFailure Enum" :default "NetDriverAlreadyExists") (bIsServer :type Boolean))
  ;[1 1 1] Muestra errores en la red
  (if bIsServer
    _
    (else
      _))
  (`self.DisplayErrorMessage` (`self.NetErrorToString` FailureType)))

(event `self.HandleTravelError`
  (params (FailureType :type "ETravelFailure Enum" :default "NoLevel"))
  ;[1 1 1] Muestra errores de conexión
  (`self.DisplayErrorMessage` (`self.TravelErrorToString` FailureType)))

(event `LaunchLobby`
  (params (NumberOfPlayers :type Integer) (`EnableLan?` :type Boolean) (ServerName :type String))
  ;[1 1 1] Ejecuta el Lobby con configuración del host
  (set `self.MaxPlayers` NumberOfPlayers)
  (set `self.ServerName` ServerName)
  (`self.ShowLoadingScreen`)
  (`CreateSessionCallbackProxy.CreateSession` (`GameplayStatics.GetPlayerController` 0) (`self.MaxPlayers`) `EnableLan?`
    (:`OnSuccess`
      (`GameplayStatics.OpenLevel` "Lobby" true "listen"))
    (:`OnFailure`
      (`self.DisplayErrorMessage` "FAILED TO CREATE SESSION, TRY AGAIN"))))

(event `ShowHostMenu`
  ;[1 1 1] Muestra el menú de crear partida online
  (`/Engine/EditorBlueprintResources/StandardMacros.IsValid` (`self.HostMenuWB`)
    (:`Is Valid`
      _)
    (:`Is Not Valid`
      (bind _returnvalue (`|CreateWidget` "/Game/UI/MainMenu/HostMenu.HostMenu_C" (`GameplayStatics.GetPlayerController` 0)))
      (set `self.HostMenuWB` _returnvalue)))
  (`UserWidget.AddToViewport` (`self.HostMenuWB`) 0))

(event `DestroySessionCaller`
  (params (PlayerController :type "PlayerController Object Reference"))
  ;[1 1 1] Destruye la sesión cuando es llamada
  (`DestroySessionCallbackProxy.DestroySession` PlayerController))

(event `ShowServerMenu`
  ;[1 1 1] Muestra el menú de servidores a conectarse
  (bind _returnvalue (`|CreateWidget` "/Game/UI/MainMenu/ServerMenu.ServerMenu_C" (`GameplayStatics.GetPlayerController` 0))) ; Como va a hacer falta regenerarlo regularmente, no se hace la comprobación previa y se envía al viewport directo
  (`UserWidget.AddToViewport` _returnvalue 0))

(event `JoinServer`
  (params (sessionToJoin :type "BlueprintSessionResult Structure"))
  ;[1 1 1] Unirse a partida
  (`self.ShowLoadingScreen`)
  (`JoinSessionCallbackProxy.JoinSession` (`GameplayStatics.GetPlayerController` 0) sessionToJoin
    (:`OnFailure`
      (`self.DisplayErrorMessage` "FAILED TO JOIN SESSION, TRY AGAIN"))))

(event `ShowOptionsMenu`
  ;[1 1 1] Muestra el menú de opciones
  (`/Engine/EditorBlueprintResources/StandardMacros.IsValid` (`self.OptionsMenuWB`)
    (:`Is Valid`
      _)
    (:`Is Not Valid`
      (bind _returnvalue (`|CreateWidget` "/Game/UI/MainMenu/OptionsMenu.OptionsMenu_C" (`GameplayStatics.GetPlayerController` 0)))
      (set `self.OptionsMenuWB` _returnvalue)))
  (`UserWidget.AddToViewport` (`self.OptionsMenuWB`) 0)
  (if (not (`self.CreatedSaveFile?`))
    (set `/Game/UI/MainMenu/OptionsMenu.WelcomeMessageVis` "Visible" (`self.OptionsMenuWB`))))

(fn `CheckSaveGame`
  (bind _returnvalue (`GameplayStatics.DoesSaveGameExist` (`self.PlayerSettingsSave`)))
  (if _returnvalue
    (`self.GameLoad`)
    (else
      (`self.GameSave`))))

(fn `GameLoad`
  (bind _returnvalue (`GameplayStatics.LoadGameFromSlot` (`self.PlayerSettingsSave`)))
  (bind _asplayer_save_game (cast `/Game/Blueprints/AllLevels/PlayerSaveGame` _returnvalue))
  (set `self.PlayerInfo` (`/Game/Blueprints/AllLevels/PlayerSaveGame.S_PlayerInfo` _asplayer_save_game)))

(fn `GameSave`
  (bind _savegameref (`self.SaveGameRef`))
  (`/Engine/EditorBlueprintResources/StandardMacros.IsValid` (`self.SaveGameRef`)
    (:`Is Valid`
      _)
    (:`Is Not Valid`
      (bind _returnvalue (`GameplayStatics.CreateSaveGameObject` "/Game/Blueprints/AllLevels/PlayerSaveGame.PlayerSaveGame_C"))
      (set `self.SaveGameRef` _returnvalue)))
  (set `/Game/Blueprints/AllLevels/PlayerSaveGame.S_PlayerInfo` (`self.PlayerInfo`) _savegameref)
  (`GameplayStatics.SaveGameToSlot` _savegameref (`self.PlayerSettingsSave`)))

(fn `NetErrorToString`
  (params (FailureType :type "ENetworkFailure Enum" :default "NetDriverAlreadyExists"))
  (returns (OutString :type String))
  (switch `ENetworkFailure` FailureType
    (:`NetDriverAlreadyExists`
      (set `self.ErrorString` "Error: Lost Connection To Host" :!label _label))
    (:`NetDriverCreateFailure`
      (goto _label))
    (:`NetDriverListenFailure`
      (goto _label))
    (:`ConnectionLost`
      (goto _label))
    (:`ConnectionTimeout`
      (set `self.ErrorString` "Error: Connection Timed Out"))
    (:`FailureReceived`
      (goto _label))
    (:`OutdatedClient`
      (goto _label))
    (:`OutdatedServer`
      (goto _label))
    (:`PendingConnectionFailure`
      (goto _label))
    (:`NetGuidMismatch`
      (goto _label))
    (:`NetChecksumMismatch`
      (goto _label)))
  (return (`self.ErrorString`)))

(fn `TravelErrorToString`
  (params (FailureType :type "ETravelFailure Enum" :default "NoLevel"))
  (returns (OutString :type String))
  (return (`KismetStringLibrary.Concat_StrStr` "Error: Failed To Travel." (`|GetEnumeratorNameAsString` FailureType))))